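; BP_PoisonTrap is an actor that deals radial poison damage around its location.
; On BeginPlay it caches the first player pawn as BP_ThirdPersonCharacter.
; Each Tick, while that character's Poison flag is set, it applies full radial damage within DamageRadius and draws a debug sphere of the same radius.
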(event `self.ReceiveBeginPlay`
  (bind _asbp_third_person_character (cast `/Game/ThirdPerson/Blueprints/BP_ThirdPersonCharacter` (`GameplayStatics.GetPlayerPawn` 0)))
  (set `self.As BP Third Person Character` _asbp_third_person_character))

(event `self.ReceiveTick`
  (params (DeltaSeconds :type "Float (single-precision)"))
  (bind _returnvalue (`self.K2_GetActorLocation`))
  (if (`/Game/ThirdPerson/Blueprints/BP_ThirdPersonCharacter.Poison` (stale `self.ReceiveBeginPlay` _asbp_third_person_character))
    (`GameplayStatics.ApplyRadialDamage` :`BaseDamage` 1.0 :`Origin` _returnvalue :`DamageRadius` (`self.Damage Radius`) :`DamageCauser` self :`InstigatedByController` null :`bDoFullDamage` true)
    (`KismetSystemLibrary.DrawDebugSphere` _returnvalue (`self.Damage Radius`) 12 (struct :`R` 0.375945 :`G` 0.418739 :`B` 1.0 :`A` 1.0) 0.0 3.0)))

(fn `UserConstructionScript`)