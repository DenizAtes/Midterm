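; BP_SpikeTrap is a spike trap that raises and damages the third-person player character when that character's Spike flag is set.
; Overlapping the Raidus component sets TrapUp and snaps Trap to a 90-degree pitch, with no reset or later read of TrapUp here.
; Any actor overlap applies fixed damage to player pawn 0, regardless of which actor overlapped or whether the trap is up.
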(event `self.ReceiveActorBeginOverlap`
  (params (OtherActor :type "Actor Object Reference"))
  (bind _asbp_third_person_character (cast `/Game/ThirdPerson/Blueprints/BP_ThirdPersonCharacter` (`GameplayStatics.GetPlayerPawn` 0)))
  (if (`/Game/ThirdPerson/Blueprints/BP_ThirdPersonCharacter.Spike` _asbp_third_person_character)
    (`GameplayStatics.ApplyDamage` _asbp_third_person_character 20.0 null self)))

(event `self.Raidus.OnComponentBeginOverlap`
  (params (OverlappedComponent :type "PrimitiveComponent Object Reference") (OtherActor :type "Actor Object Reference") (OtherComp :type "PrimitiveComponent Object Reference") (OtherBodyIndex :type Integer) (bFromSweep :type Boolean) (SweepResult :type "HitResult Structure (by ref)"))
  (bind _asbp_third_person_character (cast `/Game/ThirdPerson/Blueprints/BP_ThirdPersonCharacter` OtherActor))
  (if (`/Game/ThirdPerson/Blueprints/BP_ThirdPersonCharacter.Spike` _asbp_third_person_character)
    (set `self.TrapUp` true)
    (`SceneComponent.K2_SetRelativeRotation` (`self.Trap`) (struct :`Roll` 90.0) false false)))

(fn `UserConstructionScript`)