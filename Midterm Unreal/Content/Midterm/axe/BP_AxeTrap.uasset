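; BP_AxeTrap is a swinging blade trap that damages the player while the third-person character's Axe flag is set.
; BeginPlay caches the player and computes a target rotation pitched -90 degrees from the start.
; While Axe is true, Tick uses a Delay to repeatedly restart the SwingBlade timeline, which lerps actor rotation; otherwise it stops the timeline.
; Overlapping the player applies damage only when Axe is true.
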(event `self.ReceiveBeginPlay`
  (bind _returnvalue (`self.K2_GetActorRotation`))
  (bind _asbp_third_person_character (cast `/Game/ThirdPerson/Blueprints/BP_ThirdPersonCharacter` (`GameplayStatics.GetPlayerPawn` 0)))
  (set `self.As BP Third Person Character` _asbp_third_person_character)
  (set `self.CurrentPos` _returnvalue)
  (set `self.SwingTo` (`KismetMathLibrary.MakeRotator` (.roll _returnvalue) (+ (.pitch _returnvalue) -90.0) (.yaw _returnvalue))))

(event `self.ReceiveTick`
  (params (DeltaSeconds :type "Float (single-precision)"))
  (if (`/Game/ThirdPerson/Blueprints/BP_ThirdPersonCharacter.Axe` (`self.As BP Third Person Character`))
    (`KismetSystemLibrary.Delay` (`self.Duration`))
    (bind (_direction _swingblade_track) (`Timeline|SwingBlade` :!via `PlayFromStart` :!label _label)
      (:`Update`
        (`self.K2_SetActorRotation` (`KismetMathLibrary.RLerp` (`self.CurrentPos`) (`self.SwingTo`) _swingblade_track))))
    (else
      (goto _label :!via `Stop`))))

(event `self.ReceiveActorBeginOverlap`
  (params (OtherActor :type "Actor Object Reference"))
  (bind _asbp_third_person_character (cast `/Game/ThirdPerson/Blueprints/BP_ThirdPersonCharacter` (`GameplayStatics.GetPlayerPawn` 0)))
  (if (and (`/Game/ThirdPerson/Blueprints/BP_ThirdPersonCharacter.Axe` _asbp_third_person_character) (== OtherActor _asbp_third_person_character))
    (`GameplayStatics.ApplyDamage` _asbp_third_person_character 50.0 null self)))

(fn `UserConstructionScript`)